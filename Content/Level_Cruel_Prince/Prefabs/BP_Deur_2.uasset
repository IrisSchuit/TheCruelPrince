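; BP_Deur_2 is a locked door in the Cruel Prince level that opens once the player character has found all needed items.
; An overlap box checks the ThirdPersonCharacter's found-item count against the required count.
; On success it plays an opening sound once and a timeline rotates the pivot from its starting rotation to world zero.
; Otherwise it plays a locked sound, only the first time.
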(event OnComponentBeginOverlap(Box)
  (params (OverlappedComponent :type Primitive%20Component%20Object%20Reference) (OtherActor :type Actor%20Object%20Reference) (OtherComp :type Primitive%20Component%20Object%20Reference) (OtherBodyIndex :type Integer) (bFromSweep :type Boolean) (SweepResult :type Hit%20Result%20Structure%20%28by%20ref%29))
  (bind _asbp_third_person_character (Utilities|Casting|CastToBP_ThirdPersonCharacter OtherActor))
  (bind _haskey (CallFunction|CheckHasKey _asbp_third_person_character))
  (if (and _haskey (not (Variables|Default|GetDoorOpened)))
    (Variables|Default|SetDoorOpened true)
    (Audio|PlaySound2D "/Game/Level_Cruel_Prince/Sounds/DeurOpen.DeurOpen" 1.0 1.0 0.0 0 0)
    (bind _opendoor (Timeline|OpenDoorTimeline Play)
      (:Update
        (Transformation|SetWorldRotation (Variables|Default|GetDeurPivot) (Math|Rotator|Lerp(Rotator) (Variables|Default|GetClosedRotation) (Variables|Default|GetOpenedRotation) _opendoor) false false)))
    (else
      (bind _haskey_2 (CallFunction|CheckHasKey _asbp_third_person_character))
      (if (and (not _haskey_2) (not (Variables|Default|GetKnowsDoorIsLocked)))
        (Audio|PlaySound2D "/Game/Level_Cruel_Prince/Sounds/DeurOpSlot.DeurOpSlot" 1.0 1.0 0.0 0 0)
        (Variables|Default|SetKnowsDoorIsLocked true)))))

(event EventBeginPlay
  (Variables|Default|SetClosedRotation (Transformation|GetWorldRotation (Variables|Default|GetDeurPivot)))
  (Variables|Default|SetOpenedRotation (Math|Rotator|MakeRotator 0.0 0.0 0.0)))

(event EventTick
  (params (DeltaSeconds :type Float%20%28single-precision%29)))

(fn ConstructionScript)

(fn CheckHasKey
  (params (BP_ThirdpersonCharacter :type BP%20Third%20Person%20Character%20Object%20Reference))
  (return (== (Variables|/Game/ThirdPerson/Blueprints/BP_ThirdPersonCharacter.BP_ThirdPersonCharacter_C|GetItemsFound BP_ThirdpersonCharacter) (Variables|/Game/ThirdPerson/Blueprints/BP_ThirdPersonCharacter.BP_ThirdPersonCharacter_C|GetItemsNeeded BP_ThirdpersonCharacter))))