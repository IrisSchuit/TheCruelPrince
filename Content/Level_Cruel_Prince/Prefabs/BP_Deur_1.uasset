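; BP_Deur_1 is a door that opens when the third-person character enters its trigger and closes when they leave.
; A timeline lerps the pivot from its starting world rotation to a fixed zero world rotation, then reverses to close.
; An animating flag ignores entries mid-swing, while exits mid-swing set a flag that defers closing until the timeline finishes.
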(event OnComponentBeginOverlap(DoorTrigger)
  (params (OverlappedComponent :type Primitive%20Component%20Object%20Reference) (OtherActor :type Actor%20Object%20Reference) (OtherComp :type Primitive%20Component%20Object%20Reference) (OtherBodyIndex :type Integer) (bFromSweep :type Boolean) (SweepResult :type Hit%20Result%20Structure%20%28by%20ref%29))
  (if (not (Variables|Default|GetIsAnimating))
    (Variables|Default|SetIsOpen false)
    (Utilities|Casting|CastToBP_ThirdPersonCharacterClass (Utilities|GetClass OtherActor))
    (bind _doorrotation (Timeline|OpenDoorTimeLine Play)
      (:Update
        (Variables|Default|SetIsAnimating true)
        (Transformation|SetWorldRotation (Variables|Default|GetDoorPivot) (Math|Rotator|Lerp(Rotator) (Variables|Default|GetClosedRotation) (Variables|Default|GetOpenedRotation) _doorrotation) false false))
      (:Finished
        (Variables|Default|SetIsAnimating false)
        (if (Variables|Default|GetShouldClose)
          (Variables|Default|SetShouldClose false)
          (Variables|Default|SetIsOpen true)
          (Utilities|Casting|CastToBP_ThirdPersonCharacterClass (Utilities|GetClass (stale OnComponentEndOverlap(DoorTrigger) OtherActor)))
          (Timeline|OpenDoorTimeLine Reverse))))))

(event OnComponentEndOverlap(DoorTrigger)
  (params (OverlappedComponent :type Primitive%20Component%20Object%20Reference) (OtherActor :type Actor%20Object%20Reference) (OtherComp :type Primitive%20Component%20Object%20Reference) (OtherBodyIndex :type Integer))
  (if (Variables|Default|GetIsAnimating)
    (Variables|Default|SetShouldClose true)
    (else
      (Variables|Default|SetIsOpen true :!label _label)
      (Utilities|Casting|CastToBP_ThirdPersonCharacterClass (Utilities|GetClass OtherActor))
      (bind _doorrotation (Timeline|OpenDoorTimeLine Reverse)
        (:Update
          (Variables|Default|SetIsAnimating true)
          (Transformation|SetWorldRotation (Variables|Default|GetDoorPivot) (Math|Rotator|Lerp(Rotator) (Variables|Default|GetClosedRotation) (Variables|Default|GetOpenedRotation) _doorrotation) false false))
        (:Finished
          (Variables|Default|SetIsAnimating false)
          (if (Variables|Default|GetShouldClose)
            (Variables|Default|SetShouldClose false)
            (goto _label)))))))

(event EventBeginPlay
  (Variables|Default|SetClosedRotation (Transformation|GetWorldRotation (Variables|Default|GetDoorPivot)))
  (Variables|Default|SetOpenedRotation (Math|Rotator|MakeRotator 0.0 0.0 0.0)))

(event Collision|EventActorBeginOverlap
  (params (OtherActor :type Actor%20Object%20Reference)))

(event EventTick
  (params (DeltaSeconds :type Float%20%28single-precision%29)))

(fn ConstructionScript)