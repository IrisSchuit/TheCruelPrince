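; Searchable level object that may randomly hold one of the items the player must find, or serve as the final clue spot.
; Its box overlap registers it with BP_ThirdPersonCharacter and toggles that character's search prompt widget.
; Interact allows one search until the quota is met, raising the character's count with a count-indexed sound or playing a not-found cue.
; Afterwards, the final item plays closing dialogue and sets character flags, one after a delay.
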(event OnComponentBeginOverlap(Boxcollision)
  (params (OverlappedComponent :type Primitive%20Component%20Object%20Reference) (OtherActor :type Actor%20Object%20Reference) (OtherComp :type Primitive%20Component%20Object%20Reference) (OtherBodyIndex :type Integer) (bFromSweep :type Boolean) (SweepResult :type Hit%20Result%20Structure%20%28by%20ref%29))
  (bind _asbp_third_person_character (Utilities|Casting|CastToBP_ThirdPersonCharacter OtherActor))
  (bind _output_get (Variables|Default|SetThirdPersonCharacter _asbp_third_person_character))
  (Variables|/Game/ThirdPerson/Blueprints/BP_ThirdPersonCharacter.BP_ThirdPersonCharacter_C|SetSearchableObject _output_get self)
  (Variables|/Game/ThirdPerson/Blueprints/BP_ThirdPersonCharacter.BP_ThirdPersonCharacter_C|SetCanSearch _asbp_third_person_character true)
  (CallFunction|ShowPrompt))

(event OnComponentEndOverlap(Boxcollision)
  (params (OverlappedComponent :type Primitive%20Component%20Object%20Reference) (OtherActor :type Actor%20Object%20Reference) (OtherComp :type Primitive%20Component%20Object%20Reference) (OtherBodyIndex :type Integer))
  (bind _asbp_third_person_character (Utilities|Casting|CastToBP_ThirdPersonCharacter OtherActor))
  (Variables|/Game/ThirdPerson/Blueprints/BP_ThirdPersonCharacter.BP_ThirdPersonCharacter_C|SetCanSearch _asbp_third_person_character false)
  (CallFunction|HidePrompt))

(event Custom|Interact
  (bind _thirdpersoncharacter (Variables|Default|GetThirdPersonCharacter))
  (if (Math|Boolean|ANDBoolean (Variables|Default|GetHasItem) (Variables|Default|GetItemNotFound) (< (Variables|/Game/ThirdPerson/Blueprints/BP_ThirdPersonCharacter.BP_ThirdPersonCharacter_C|GetItemsFound (Variables|Default|GetThirdPersonCharacter)) (Variables|/Game/ThirdPerson/Blueprints/BP_ThirdPersonCharacter.BP_ThirdPersonCharacter_C|GetItemsNeeded (Variables|Default|GetThirdPersonCharacter))))
    (bind _output_get (Variables|/Game/ThirdPerson/Blueprints/BP_ThirdPersonCharacter.BP_ThirdPersonCharacter_C|SetItemsFound (Variables|Default|GetThirdPersonCharacter) (+ 1 (Variables|/Game/ThirdPerson/Blueprints/BP_ThirdPersonCharacter.BP_ThirdPersonCharacter_C|GetItemsFound (Variables|Default|GetThirdPersonCharacter)))))
    (CallFunction|PlayItemFoundSound)
    (Development|PrintString (Utilities|String|ToString(Integer) _output_get))
    (Variables|Default|SetItemNotFound false)
    (CallFunction|HidePrompt :!label _label)
    (elif (< (Variables|/Game/ThirdPerson/Blueprints/BP_ThirdPersonCharacter.BP_ThirdPersonCharacter_C|GetItemsFound (Variables|Default|GetThirdPersonCharacter)) (Variables|/Game/ThirdPerson/Blueprints/BP_ThirdPersonCharacter.BP_ThirdPersonCharacter_C|GetItemsNeeded (Variables|Default|GetThirdPersonCharacter)))
      (if (Variables|Default|GetItemNotFound)
        (Audio|PlaySound2D "/Game/Level_Cruel_Prince/Sounds/NotFoundSoundCue.NotFoundSoundCue" 1.0 1.0 0.0 0 0)
        (Variables|Default|SetItemNotFound false)
        (goto _label))
      (elif (Variables|Default|GetisFinalItem)
        (Audio|PlaySound2D "/Game/Level_Cruel_Prince/Sounds/LaatsteClueBoven.LaatsteClueBoven" 1.0 1.0 0.0 0 0)
        (CallFunction|HidePrompt)
        (Audio|PlaySound2D "/Game/Level_Cruel_Prince/Sounds/VerstopJeBoven.VerstopJeBoven" 1.0 1.0 0.0 0 0)
        (Variables|/Game/ThirdPerson/Blueprints/BP_ThirdPersonCharacter.BP_ThirdPersonCharacter_C|SetFoundFinalClue _thirdpersoncharacter true)
        (Utilities|FlowControl|Delay 22.0)
        (Variables|/Game/ThirdPerson/Blueprints/BP_ThirdPersonCharacter.BP_ThirdPersonCharacter_C|SetIsDoneWithFinalDialogue _thirdpersoncharacter true)))))

(event EventBeginPlay
  (Variables|Default|SetHasItem (Math|Random|RandomBool))
  (Variables|Default|SetItemNotFound true))

(event Collision|EventActorBeginOverlap
  (params (OtherActor :type Actor%20Object%20Reference)))

(event EventTick
  (params (DeltaSeconds :type Float%20%28single-precision%29)))

(fn ConstructionScript)

(fn ShowPrompt
  (bind _thirdpersoncharacter (Variables|Default|GetThirdPersonCharacter))
  (bind _itemnotfound (Variables|Default|GetItemNotFound))
  (if (and (not (== (Variables|/Game/ThirdPerson/Blueprints/BP_ThirdPersonCharacter.BP_ThirdPersonCharacter_C|GetItemsFound _thirdpersoncharacter) (Variables|/Game/ThirdPerson/Blueprints/BP_ThirdPersonCharacter.BP_ThirdPersonCharacter_C|GetItemsNeeded _thirdpersoncharacter))) _itemnotfound)
    (Variables|/Script/UMG.Widget|SetVisibility (UserInterface|GetWidget (Variables|/Game/ThirdPerson/Blueprints/BP_ThirdPersonCharacter.BP_ThirdPersonCharacter_C|GetSearchingPromptWidget (Variables|Default|GetThirdPersonCharacter))) "Visible" :!label _label)
    (elif (and (Variables|Default|GetisFinalItem) _itemnotfound)
      (goto _label))))

(fn HidePrompt
  (Variables|/Script/UMG.Widget|SetVisibility (UserInterface|GetWidget (Variables|/Game/ThirdPerson/Blueprints/BP_ThirdPersonCharacter.BP_ThirdPersonCharacter_C|GetSearchingPromptWidget (Variables|Default|GetThirdPersonCharacter))) "Hidden"))

(fn PlayItemFoundSound
  (Audio|PlaySound2D (Utilities|Array|Get(acopy) (Variables|Default|GetItemFoundSounds) (- (Variables|/Game/ThirdPerson/Blueprints/BP_ThirdPersonCharacter.BP_ThirdPersonCharacter_C|GetItemsFound (Variables|Default|GetThirdPersonCharacter)) 1)) 1.0 1.0 0.0 0 0))