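; BP_Spooky is a recurring hide-check scare event for the Cruel Prince level.
; A looping timer, its interval randomized once at BeginPlay, plays a hiding cue and repeats footsteps audio three times via a delayed loop.
; It then reads IsHidden on the player character's BlackScreenWidget to play either a revealing cue or a found sound, printing "Game over" for the latter.
; A ReadyToPlay flag blocks overlapping runs.
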(event Custom|StartMusic
  (if (Variables|Default|GetReadyToPlay)
    (Variables|Default|SetReadyToPlay false)
    (Audio|PlaySound2D "/Game/Level_Cruel_Prince/Sounds/HiddingCue.HiddingCue" 1.0 1.0 0.0 0 0)
    (bind _result (Math|Integer|IncrementInt (Variables|Default|GetPlayCount) :!label _label)
      (:%20%20
        (bind _output_get (Variables|Default|SetPlayCount _result))
        (if (<= _output_get 3)
          (Audio|Components|Audio|Play (Variables|Default|GetFootsteps_Audio) 0.0)
          (Utilities|FlowControl|Delay 2.45)
          (goto _label)
          (else
            (Variables|Default|SetReadyToPlay true)
            (Variables|Default|SetPlayCount 0)
            (bind _outactors (Actor|GetAllActorsOfClass "/Game/ThirdPerson/Blueprints/BP_ThirdPersonCharacter.BP_ThirdPersonCharacter_C"))
            (bind _output_get_2 (Variables|Default|SetBlackScreenWidget (Variables|/Game/ThirdPerson/Blueprints/BP_ThirdPersonCharacter.BP_ThirdPersonCharacter_C|GetBlackScreenWidget (Utilities|Array|Get(acopy) _outactors))))
            (if (Variables|/Game/Level_Cruel_Prince/Prefabs/BlackScreenWidget.BlackScreenWidget_C|GetisHidden _output_get_2)
              (Development|PrintString "Hidden")
              (Audio|PlaySound2D "/Game/Level_Cruel_Prince/Sounds/RevealingSoundCue.RevealingSoundCue" 1.0 1.0 0.0 0 0)
              (else
                (Development|PrintString "Game over")
                (Audio|PlaySound2D "/Game/Level_Cruel_Prince/Sounds/GevondenBoven.GevondenBoven" 1.0 1.0 0.0 0 0)))))))))

(event EventBeginPlay
  (Utilities|Time|SetTimerbyEvent (delegate Custom|StartMusic) (Math|Random|RandomFloatinRange 15.0 3e+01) true))

(event Collision|EventActorBeginOverlap
  (params (OtherActor :type Actor%20Object%20Reference)))

(event EventTick
  (params (DeltaSeconds :type Float%20%28single-precision%29)))

(fn ConstructionScript)